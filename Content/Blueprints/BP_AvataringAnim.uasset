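; Actor that shows a Kinect-driven avatar for the body number held in its Body variable.
; Each Tick it checks the Kinect's tracked bodies and scales the skeletal mesh to zero when that body is absent.
; When tracked, it passes Body to the AvataringAnim instance as CenteredBody and moves the root to the SpineBase joint with a Z offset.
; The Kinect's centered body is only printed for debugging.
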(event EventBeginPlay)

(event Collision|EventActorBeginOverlap
  (params (OtherActor :type Actor%20Object%20Reference)))

(event EventTick
  (params (DeltaSeconds :type Float%20%28single-precision%29))
  (bind _body (Variables|Default|Getbody))
  (bind _skeletalmesh (Variables|Default|GetSkeletalMesh))
  (bind _body_2 (Class|KinectDeviceComponent|GetCenteredBody (Variables|Default|GetKinectDevice)))
  (Development|PrintString (Utilities|String|EnumtoString _body_2))
  (bind _tracked (CallFunction|IsTracked))
  (if _tracked
    (Transformation|SetWorldScale3D _skeletalmesh "1.000000,1.000000,1.000000")
    (bind _asavataring_anim (Utilities|Casting|CastToAvataringAnim (Components|SkeletalMesh|GetAnimInstance _skeletalmesh)))
    (Variables|/Game/Blueprints/AvataringAnim.AvataringAnim_C|SetCenteredBody _asavataring_anim _body)
    (bind _returnvalue (Class|KinectDeviceComponent|GetJointAbsolutePosition (Variables|Default|GetKinectDevice) "SpineBase" _body))
    (Transformation|SetWorldTransform (Variables|Default|GetDefaultSceneRoot) (Math|Transform|MakeTransform (Math|Vector|MakeVector (.X (Math|Vector|BreakVector _returnvalue)) (.Y (Math|Vector|BreakVector _returnvalue)) (+ (.Z (Math|Vector|BreakVector _returnvalue)) 5e+01)) "0, 0, 0" "1,1,1") false false)
    (else
      (Transformation|SetWorldScale3D _skeletalmesh "0, 0, 0"))))

(fn ConstructionScript)

(fn IsTracked
  (bind _body (Class|KinectDeviceComponent|GetTrackedBodies (Variables|Default|GetKinectDevice)))
  (for _array_element _body
    (if (== _array_element (Variables|Default|Getbody))
      (return true)))
  (return false))